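; Zombie enemy that wanders the navmesh until it spots a pawn, then hunts the player.
; Tick-driven patrol picks random reachable points around its current location.
; PawnSensing ends patrol, sets chase speed and starts an AI MoveTo loop that retries on failure and alternates with attack montages.
; Player bullet hits on the capsule reduce health; at zero it clears the Alive flag here and in ABP_Zombie.
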(event OnComponentHit(CapsuleComponent)
  (params (HitComponent :type Primitive%20Component%20Object%20Reference) (OtherActor :type Actor%20Object%20Reference) (OtherComp :type Primitive%20Component%20Object%20Reference) (NormalImpulse :type Vector :default "0, 0, 0") (Hit :type Hit%20Result%20Structure%20%28by%20ref%29))
  ;[1 1 1] BulletHIt
  (bind _asbp_player_bullet (Utilities|Casting|CastToBP_PlayerBullet OtherActor))
  (CallFunction|TakeDamage (Variables|/Game/Blueprints/Weapons/Bullet/BP_Bullet.BP_Bullet_C|GetDamage _asbp_player_bullet)))

(event OnSeePawn(PawnSensing)
  (params (Pawn :type Pawn%20Object%20Reference))
  ;[1 1 1] OnSeePawn
  (if (Variables|Default|GetAlive)
    (Variables|/Script/Engine.CharacterMovementComponent|SetMaxWalkSpeed (Variables|Character|GetCharacterMovement) 3e+02)
    (Variables|Patrol|SetEnablePatrol false)
    (if (not (Variables|Default|GetPlayerFound))
      (Variables|Default|SetPlayerFound true)
      (CallFunction|MovetoPlayer))))

(event Custom|MoveToPlayer
  ;[1 1 1] MoveToPlayer
  (if (Variables|Default|GetAlive)
    (AI|AIMoveTo self "0, 0, 0" (Game|Player|GetPlayerPawn 0) 4e+01 false
      (:OnSuccess
        (CallFunction|AttackPlayer))
      (:OnFail
        (CallFunction|MovetoPlayer)))))

(event Custom|AttackPlayer
  ;[1 1 1] AttackPlayer
  (if (Variables|Default|GetAlive)
    (Animation|Montage|PlayMontage (Variables|Character|GetMesh) "/Game/Models/Enemies/ZombieGirl/Animations/AM_ZombieAttack.AM_ZombieAttack"
      (:OnCompleted
        (CallFunction|MovetoPlayer)))))

(event Custom|Patrol
  ;[1 1 1] Patrol
  (if (Variables|Patrol|GetTargetReached)
    (bind _target (CallFunction|GetNewPatrolLocation))
    (AI|AIMoveTo self _target 0 5.0 false)
    (elif (CallFunction|PatrolPointReached)
      (Variables|Patrol|SetTargetReached true))))

(event EventBeginPlay)

(event Collision|EventActorBeginOverlap
  (params (OtherActor :type Actor%20Object%20Reference)))

(event EventTick
  (params (DeltaSeconds :type Float%20%28single-precision%29))
  (if (Variables|Patrol|GetEnablePatrol)
    (CallFunction|Patrol)))

(fn ConstructionScript)

(fn TakeDamage
  (params (Damage :type Integer))
  (bind _output_get (Variables|Default|SetHealth (- (Variables|Default|GetHealth) Damage)))
  (if (<= _output_get 0)
    (bind _asabp_zombie (Utilities|Casting|CastToABP_Zombie (Components|SkeletalMesh|GetAnimInstance (Variables|Character|GetMesh))))
    (Variables|/Game/Blueprints/Enemies/Zombie/ABP_Zombie.ABP_Zombie_C|SetAlive _asabp_zombie false)
    (Variables|Default|SetAlive false)))

(fn GetNewPatrolLocation
  (bind _randomlocation (Class|NavigationSystemV1|GetRandomLocationinNavigableRadius (Transformation|GetActorLocation) 5e+03 0 0))
  (Variables|Patrol|SetTarget _randomlocation)
  (Variables|Patrol|SetTargetReached false)
  (return (Variables|Patrol|GetTarget)))

(fn PatrolPointReached
  (return (<= (Math|Vector|Distance(Vector) (Transformation|GetActorLocation) (Variables|Patrol|GetTarget)) 1e+02)))