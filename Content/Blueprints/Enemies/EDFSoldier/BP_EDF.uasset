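; EDF soldier enemy that patrols random navmesh points until pawn sensing spots a pawn, then permanently switches to hunting the player.
; Each tick it traces to the player camera, then either chases or, within shooting distance, stops, faces and aims.
; Shooting and aim state drive AB_EDFSoldier; ShootPlayer spawns muzzle flash and bullet but isn't called in this Blueprint.
; The bullet-hit death logic is disconnected.
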(event OnSeePawn(PawnSensing)
  (params (Pawn :type Pawn%20Object%20Reference))
  (if (not (Variables|Default|GetPlayerFound))
    (Variables|Default|SetPlayerFound true)
    (bind _asab_edfsoldier (Utilities|Casting|CastToAB_EDFSoldier (Components|SkeletalMesh|GetAnimInstance (Variables|Character|GetMesh))))
    (bind _aim (Timeline|Timeline_0 Play)
      (:Update
        (Variables|/Game/Characters/EDFSoldiers/Animations/AB_EDFSoldier.AB_EDFSoldier_C|SetBehaviour _asab_edfsoldier _aim)
        (Variables|/Script/Engine.CharacterMovementComponent|SetMaxWalkSpeed (Variables|Character|GetCharacterMovement) 3e+02)))))

(event OnComponentHit(CapsuleComponent)
  (params (HitComponent :type Primitive%20Component%20Object%20Reference) (OtherActor :type Actor%20Object%20Reference) (OtherComp :type Primitive%20Component%20Object%20Reference) (NormalImpulse :type Vector :default "0, 0, 0") (Hit :type Hit%20Result%20Structure%20%28by%20ref%29)))

(event Custom|Patrol
  ;[1 1 1] Patrol
  (if (Variables|Default|GetTargetReached)
    (bind _target (CallFunction|GetNewPatrolLocation))
    (AI|AIMoveTo self _target 0 5.0 false)
    (elif (CallFunction|PatrolPointReached)
      (Variables|Default|SetTargetReached true))))

(event EventTick
  (params (DeltaSeconds :type Float%20%28single-precision%29))
  (bind _muzzle (Variables|Default|GetMuzzle))
  (bind _returnvalue (Transformation|GetWorldLocation _muzzle))
  (Collision|LineTraceByChannel _returnvalue (+ _returnvalue (* (Math|Vector|GetForwardVector _muzzle) 2000)) "TraceTypeQuery1" false 0 "None")
  (if (Variables|Default|GetPlayerFound)
    ;[1 1 1] Hunt Player
    (bind (_outhit _returnvalue_2) (Collision|LineTraceByChannel (Transformation|GetActorLocation) (Transformation|GetWorldLocation (Variables|/Script/Engine.PlayerCameraManager|GetTransformComponent (Game|GetPlayerCameraManager 0))) "TraceTypeQuery2" false 0 "None"))
    (if _returnvalue_2
      (if (Actor|ActorHasTag (.HitActor (Collision|BreakHitResult _outhit)) "Player")
        (if (<= (Math|Vector|Distance(Vector) (Transformation|GetActorLocation (.HitActor (Collision|BreakHitResult _outhit))) (Transformation|GetActorLocation)) (Variables|Default|GetShootingDistance))
          (Components|Movement|StopMovementImmediately (Variables|Character|GetCharacterMovement))
          (CallFunction|LookatPlayer)
          (CallFunction|SetAimRotation 0.15)
          (CallFunction|PlayShootAnimation true)
          (else
            (CallFunction|SetAimRotation 0.0)
            (CallFunction|PlayShootAnimation false)
            (AI|AIMoveTo self "0, 0, 0" (.HitActor (Collision|BreakHitResult _outhit)) 5.0 false)))
        (else
          (CallFunction|PlayShootAnimation false :!label _label)))
      (else
        (goto _label)))
    (else
      (CallFunction|Patrol))))

(fn ConstructionScript)

(fn PlayShootAnimation
  (params (Shoot :type Boolean))
  (bind _asab_edfsoldier (Utilities|Casting|CastToAB_EDFSoldier (Components|SkeletalMesh|GetAnimInstance (Variables|Character|GetMesh))))
  (Variables|/Game/Characters/EDFSoldiers/Animations/AB_EDFSoldier.AB_EDFSoldier_C|SetShootPlayer _asab_edfsoldier Shoot))

(fn SetAimRotation
  (params (AimOffset :type Float%20%28double-precision%29))
  (bind _asab_edfsoldier (Utilities|Casting|CastToAB_EDFSoldier (Components|SkeletalMesh|GetAnimInstance (Variables|Character|GetMesh))))
  (Variables|/Game/Characters/EDFSoldiers/Animations/AB_EDFSoldier.AB_EDFSoldier_C|SetAimRotation _asab_edfsoldier (Math|Rotator|MakeRotator (* (.z (- (Transformation|GetActorLocation) (Transformation|GetWorldLocation (Variables|/Script/Engine.PlayerCameraManager|GetTransformComponent (Game|GetPlayerCameraManager 0))))) AimOffset) -2e+01 0.0)))

(fn ShootPlayer
  (bind _muzzle (Variables|Default|GetMuzzle))
  (bind _returnvalue (Transformation|GetWorldLocation _muzzle))
  (bind _returnvalue_2 (Transformation|GetWorldRotation _muzzle))
  (if (Variables|Default|GetAlive)
    (Effects|SpawnEmitteratLocation "/Game/MilitaryWeapSilver/FX/P_AssaultRifle_MuzzleFlash.P_AssaultRifle_MuzzleFlash" _returnvalue _returnvalue_2)
    (bind _returnvalue_3 (Game|SpawnActorfromClass "/Game/Blueprints/Weapons/Bullet/BP_EnemyBullet.BP_EnemyBullet_C" (Math|Transform|MakeTransform _returnvalue _returnvalue_2) "Undefined" 0 0))
    (Default|LaunchBullet _returnvalue_3 (Math|Vector|GetForwardVector _muzzle))))

(fn LookatPlayer
  (bind _returnvalue (Game|Player|GetPlayerPawn 0))
  (bind _returnvalue_2 (Transformation|GetActorLocation))
  (bind _returnvalue_3 (Transformation|GetActorLocation _returnvalue))
  (bind _returnvalue_4 (Math|Rotator|FindLookatRotation _returnvalue_2 _returnvalue_3))
  (Transformation|SetWorldRotation (Variables|Collision|GetCapsuleComponent) (Math|Rotator|MakeRotator (.roll _returnvalue_4) 0.0 (.yaw _returnvalue_4)) false false))

(fn GetNewPatrolLocation
  (bind _randomlocation (Class|NavigationSystemV1|GetRandomLocationinNavigableRadius (Transformation|GetActorLocation) 5e+03 0 0))
  (Variables|Default|SetTarget _randomlocation)
  (Variables|Default|SetTargetReached false)
  (return (Variables|Default|GetTarget)))

(fn PatrolPointReached
  (return (<= (Math|Vector|Distance(Vector) (Transformation|GetActorLocation) (Variables|Default|GetTarget)) 1e+02)))