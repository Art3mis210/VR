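; BP_NaziOfficer is a snow level enemy NPC that aims and plays shooting animation when it sees a pawn.
; First sighting runs a timeline that blends Behaviour on AB_NaziOfficer; later sightings turn the capsule toward the player, set ShootPlayer and derive AimRotation from camera height.
; ShootPlayer spawns only a muzzle flash and is not called within this Blueprint.
; Tick line-traces from the muzzle without using the result.
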(event OnSeePawn(PawnSensing)
  (params (Pawn :type Pawn%20Object%20Reference))
  (bind _returnvalue (Game|Player|GetPlayerPawn 0))
  (bind _returnvalue_2 (Transformation|GetActorLocation))
  (bind _returnvalue_3 (Transformation|GetActorLocation _returnvalue))
  (bind _returnvalue_4 (Math|Rotator|FindLookatRotation _returnvalue_2 _returnvalue_3))
  (if (Variables|Default|GetPlayerFound)
    (Transformation|SetWorldRotation (Variables|Collision|GetCapsuleComponent) (Math|Rotator|MakeRotator (.roll _returnvalue_4) 0.0 (.yaw _returnvalue_4)) false false)
    (CallFunction|PlayShootAnimation true)
    (CallFunction|SetAimRotation)
    (else
      (Variables|Default|SetPlayerFound true)
      (bind _asab_nazi_officer (Utilities|Casting|CastToAB_NaziOfficer (Components|SkeletalMesh|GetAnimInstance (Variables|Character|GetMesh))))
      (bind _aim (Timeline|Timeline Play)
        (:Update
          (Variables|/Game/Characters/SnowLevel/NaziOfficer/Animations/AB_NaziOfficer.AB_NaziOfficer_C|SetBehaviour _asab_nazi_officer _aim))))))

(event EventTick
  (params (DeltaSeconds :type Float%20%28single-precision%29))
  (bind _muzzle (Variables|Default|GetMuzzle))
  (bind _returnvalue (Transformation|GetWorldLocation _muzzle))
  (Collision|LineTraceByChannel _returnvalue (+ _returnvalue (* (Math|Vector|GetForwardVector _muzzle) 2000)) "TraceTypeQuery1" false 0 "None"))

(fn ConstructionScript)

(fn PlayShootAnimation
  (params (Shoot :type Boolean))
  (bind _asab_nazi_officer (Utilities|Casting|CastToAB_NaziOfficer (Components|SkeletalMesh|GetAnimInstance (Variables|Character|GetMesh))))
  (Variables|/Game/Characters/SnowLevel/NaziOfficer/Animations/AB_NaziOfficer.AB_NaziOfficer_C|SetShootPlayer _asab_nazi_officer Shoot))

(fn SetAimRotation
  (bind _asab_nazi_officer (Utilities|Casting|CastToAB_NaziOfficer (Components|SkeletalMesh|GetAnimInstance (Variables|Character|GetMesh))))
  (Variables|/Game/Characters/SnowLevel/NaziOfficer/Animations/AB_NaziOfficer.AB_NaziOfficer_C|SetAimRotation _asab_nazi_officer (Math|Rotator|MakeRotator (* (.z (- (Transformation|GetWorldLocation (Variables|/Script/Engine.PlayerCameraManager|GetTransformComponent (Game|GetPlayerCameraManager 0))) (Transformation|GetActorLocation))) (Variables|Default|GetAimOffset)) -4e+01 0.0)))

(fn NewFunction)

(fn ShootPlayer
  (bind _muzzle (Variables|Default|GetMuzzle))
  (Effects|SpawnEmitteratLocation "/Game/MilitaryWeapSilver/FX/P_AssaultRifle_MuzzleFlash.P_AssaultRifle_MuzzleFlash" (Transformation|GetWorldLocation _muzzle) (Transformation|GetWorldRotation _muzzle)))