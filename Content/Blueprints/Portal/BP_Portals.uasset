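; BP_Portals is an actor holding a pair of linked portals that teleport overlapping actors between two planes.
; Entering either plane moves the actor to the other, using that plane's yaw and the player pawn's pitch and roll.
; A shared CanTeleport flag with a one-second delay prevents instant bounce-back, and both scene captures refresh on each teleport.
; TurnOnPortals unhides the whole component hierarchy.
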(event OnComponentBeginOverlap(Plane)
  (params (OverlappedComponent :type Primitive%20Component%20Object%20Reference) (OtherActor :type Actor%20Object%20Reference) (OtherComp :type Primitive%20Component%20Object%20Reference) (OtherBodyIndex :type Integer) (bFromSweep :type Boolean) (SweepResult :type Hit%20Result%20Structure%20%28by%20ref%29))
  (bind _returnvalue (Game|Player|GetPlayerPawn 0))
  (bind _returnvalue_2 (Transformation|GetActorRotation _returnvalue))
  ;[1 1 1] Portal1Enter
  (if (Variables|Default|GetcanTeleport)
    (Variables|Default|SetcanTeleport false)
    (Transformation|SetActorLocationAndRotation OtherActor (Transformation|GetWorldLocation (Variables|Default|GetPlane1)) (Math|Rotator|MakeRotator (.roll _returnvalue_2) (.pitch _returnvalue_2) (.yaw (Transformation|GetWorldRotation (Variables|Default|GetPlane1)))))
    (CallFunction|CaptureScene)
    (Utilities|FlowControl|Delay 1.0)
    (Variables|Default|SetcanTeleport true)))

(event OnComponentBeginOverlap(Plane1)
  (params (OverlappedComponent :type Primitive%20Component%20Object%20Reference) (OtherActor :type Actor%20Object%20Reference) (OtherComp :type Primitive%20Component%20Object%20Reference) (OtherBodyIndex :type Integer) (bFromSweep :type Boolean) (SweepResult :type Hit%20Result%20Structure%20%28by%20ref%29))
  (bind _returnvalue (Game|Player|GetPlayerPawn 0))
  (bind _returnvalue_2 (Transformation|GetActorRotation _returnvalue))
  ;[1 1 1] Portal2Enter
  (if (Variables|Default|GetcanTeleport)
    (Variables|Default|SetcanTeleport false)
    (Transformation|SetActorLocationAndRotation OtherActor (Transformation|GetWorldLocation (Variables|Default|GetPlane)) (Math|Rotator|MakeRotator (.roll _returnvalue_2) (.pitch _returnvalue_2) (.yaw (Transformation|GetWorldRotation (Variables|Default|GetPlane)))))
    (CallFunction|CaptureScene)
    (Utilities|FlowControl|Delay 1.0)
    (Variables|Default|SetcanTeleport true)))

(fn ConstructionScript)

(fn CaptureScene
  (Rendering|SceneCapture|CaptureScene (Variables|Default|GetSceneCaptureComponent2D) :!class /Script/Engine.SceneCaptureComponent2D)
  (Rendering|SceneCapture|CaptureScene (Variables|Default|GetSceneCaptureComponent2D1) :!class /Script/Engine.SceneCaptureComponent2D))

(fn TurnonPortals
  (Development|SetHiddeninGame (Variables|Default|GetDefaultSceneRoot) false true))