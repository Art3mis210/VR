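; BP_Bullet is a bullet actor launched as a physics impulse on its BulletCollider.
; LaunchBullet scales the supplied vector into that impulse, while the ProjectileMovement component goes unused.
; A hit prints the other actor's name and destroys the bullet.
; An overlap prints debug text, sets Tags and turns off further overlap events on the collider, leaving the bullet alive.
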(event OnComponentHit(BulletCollider)
  (params (HitComponent :type Primitive%20Component%20Object%20Reference) (OtherActor :type Actor%20Object%20Reference) (OtherComp :type Primitive%20Component%20Object%20Reference) (NormalImpulse :type Vector :default "0, 0, 0") (Hit :type Hit%20Result%20Structure%20%28by%20ref%29))
  (Development|PrintString (Utilities|GetDisplayName OtherActor))
  (Actor|DestroyActor))

(event OnComponentBeginOverlap(BulletCollider)
  (params (OverlappedComponent :type Primitive%20Component%20Object%20Reference) (OtherActor :type Actor%20Object%20Reference) (OtherComp :type Primitive%20Component%20Object%20Reference) (OtherBodyIndex :type Integer) (bFromSweep :type Boolean) (SweepResult :type Hit%20Result%20Structure%20%28by%20ref%29))
  (Development|PrintString (Utilities|GetDisplayName OtherComp))
  (Variables|Default|SetTags (Variables|Default|GetTags_0))
  (Variables|/Script/Engine.PrimitiveComponent|SetbGenerateOverlapEvents (Variables|Default|GetBulletCollider) false)
  (Development|PrintString "Hello"))

(event EventBeginPlay)

(event Collision|EventActorBeginOverlap
  (params (OtherActor :type Actor%20Object%20Reference)))

(event EventTick
  (params (DeltaSeconds :type Float%20%28single-precision%29)))

(fn ConstructionScript)

(fn LaunchBullet
  (params (A :type Vector))
  (Physics|AddImpulse (Variables|Default|GetBulletCollider) (* A 1000) "None" false))