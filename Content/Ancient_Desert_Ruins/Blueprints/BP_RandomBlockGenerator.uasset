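; Procedural block wall generator that builds rows of damaged stone block meshes in the construction script from a seeded random stream.
; Each row draws random widths, rescales them to a fixed total, and accumulates half-widths into block centres so they sit end to end.
; Blocks get random quarter-turn yaw, while depth jitter, pitch and roll are zeroed out.
; A MultiGate for mixing in an intact block mesh is left unconnected.
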(event EventBeginPlay)

(event Collision|EventActorBeginOverlap
  (params (OtherActor :type Actor%20Object%20Reference)))

(event EventTick
  (params (DeltaSeconds :type Float%20%28single-precision%29)))

(fn ConstructionScript
  (bind _myrandomstream (Variables|Default|GetmyRandomStream))
  (for _index (range 0 (+ (Variables|Default|GetNumofHigh) -1))
    (Variables|Default|SetHeightpos (* _index (Variables|Default|GetHeightofcomponent)))
    (bind _random_numbers (CallFunction|Createrandomarray (Variables|Default|GetMinscale) (Variables|Default|GetMaxscale) (Variables|Default|GetNumofLong) (Variables|Default|GetmyRandomStream)))
    (bind _scaledfloats (CallFunction|Scalearray _random_numbers (Math|Conversions|ToFloat(Integer) (Variables|Default|GetNumofLong))))
    (Variables|Default|SetCompScaleValues _scaledfloats)
    (bind _scaledfloats_2 (CallFunction|Scalearray _random_numbers (* (Variables|Default|GetNumofLong) (Variables|Default|GetLenghtofcomponent))))
    (bind _returnvalues (CallFunction|CompPositions _scaledfloats_2))
    (Variables|Default|SetThecomppositions _returnvalues)
    (for _index_2 (range 0 (+ (Variables|Default|GetNumofLong) -1))
      (bind _returnvalue (AddComponent|AddStaticMeshComponent false (Math|Transform|MakeTransform (Math|Vector|MakeVector (Utilities|Array|Get(acopy) (Variables|Default|GetThecomppositions) _index_2) (* (Math|Random|RandomIntegerinRangefromStream -10 10 (Variables|Default|GetmyRandomStream)) 0.0) (Variables|Default|GetHeightpos)) (Math|Rotator|MakeRotator (* (Math|Random|RandomIntegerinRangefromStream 0 1 _myrandomstream) 0.0) (* (Math|Random|RandomIntegerinRangefromStream 0 1 _myrandomstream) 0.0) (* (Math|Random|RandomIntegerinRangefromStream 0 3 _myrandomstream) 9e+01)) (Math|Vector|MakeVector (Utilities|Array|Get(acopy) (Variables|Default|GetCompScaleValues) _index_2) 1.0 1.0))))
      ;[0.02718 1 0] Mesh Section
      (Components|StaticMesh|SetStaticMesh _returnvalue "/Game/Ancient_Desert_Ruins/Models/SM_Block_Damaged.SM_Block_Damaged"))))

(fn Createrandomarray
  (params (Minvalue :type Float%20%28single-precision%29) (Maxvalue :type Float%20%28single-precision%29) (Elements%20Number :type Integer) (RandomStream :type Random%20Stream%20Structure%20%28by%20ref%29))
  (for _index (range 0 (- Elements%20Number 1))
    (Utilities|Array|Add (LocalVariables|GetReturnarray) (Math|Random|RandomFloatinRangefromStream Minvalue Maxvalue RandomStream)))
  (return (LocalVariables|GetReturnarray)))

(fn PrintArray
  (params (InputArray :type Array%20of%20Floats%20%28single-precision%29))
  (Development|PrintString "-------")
  (for _array_element InputArray
    (Development|PrintString (Utilities|String|ToString(Float) _array_element)))
  (Development|PrintString "***************"))

(fn Scalearray
  (params (RandomArrayInput :type Array%20of%20Floats%20%28single-precision%29) (Targetzum :type Float%20%28single-precision%29))
  (LocalVariables|SetInputsum 0.0)
  (for _array_element RandomArrayInput
    (LocalVariables|SetInputsum (+ (LocalVariables|GetInputsum) _array_element)))
  (LocalVariables|SetScalefactor (/ Targetzum (LocalVariables|GetInputsum)))
  (for _array_element_2 RandomArrayInput
    (Utilities|Array|Add (LocalVariables|GetReturnarray) (* _array_element_2 (LocalVariables|GetScalefactor))))
  (return (LocalVariables|GetReturnarray)))

(fn CompPositions
  (params (RockSizes :type Array%20of%20Floats%20%28single-precision%29))
  (LocalVariables|SetcurrentTotel 0.0)
  (LocalVariables|SetprevElement 0.0)
  (for _array_element RockSizes
    (Utilities|FlowControl|Sequence
      (:then_0
        (LocalVariables|SetnewElement _array_element)
        (LocalVariables|SetnewTotal (|(oldTotal+(0.500000*(newaElement+prevaElement))) (LocalVariables|GetcurrentTotel) (LocalVariables|GetnewElement) (LocalVariables|GetprevElement)))
        (Utilities|Array|Add (LocalVariables|GetReturnArray) (LocalVariables|GetnewTotal)))
      (:then_1
        (LocalVariables|SetcurrentTotel (LocalVariables|GetnewTotal))
        (LocalVariables|SetprevElement (LocalVariables|GetnewElement)))))
  (return (LocalVariables|GetReturnArray)))